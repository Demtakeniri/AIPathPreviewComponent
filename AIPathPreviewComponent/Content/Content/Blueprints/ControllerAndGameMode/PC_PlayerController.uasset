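; Example player controller that previews a movement path to the cursor and drives a BP_CameraPawn through Enhanced Input.
; Tick redraws the externally set PathPreviewComp from its owner to the cursor hit, past a mouse-distance threshold with AlwaysShow, otherwise on Space.
; Releasing or canceling IA_Move fires MoveToLocation, bound in BP_Character, with the last stored cursor location.
; IA_MoveX/Y move the camera pawn along its forward/right axes and recheck height.
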(event `self.ReceiveBeginPlay`
  (`EnhancedInputSubsystemInterface.AddMappingContext` (pcsubsystem `EnhancedInputLocalPlayerSubsystem` self) "/AIPathPreviewComponent/Content/Inputs/IMC_MappingContext.IMC_MappingContext" 0 (struct))
  (bind _asbp_camera_pawn (cast `/AIPathPreviewComponent/Content/Blueprints/BP_CameraPawn` (`self.K2_GetPawn`)))
  (set `self.CameraPawn` _asbp_camera_pawn))

(event `EnhancedInput|/AIPathPreviewComponent/Content/Inputs/IA_Move`
  (params (ActionValue :type Boolean) (ElapsedSeconds :type "Float (double-precision)") (TriggeredSeconds :type "Float (double-precision)") (InputAction :type "InputAction Object Reference" :default "/AIPathPreviewComponent/Content/Inputs/IA_Move.IA_Move"))
  ;[1 1 1] Call movement event (check BP_Character tosee how the event is binded )
  (:`Canceled`
    (`self.MoveToLocation` (`self.PreviousMouseLoc`) :!label _label))
  (:`Completed`
    (goto _label)))

(event `self.ReceiveTick`
  (params (DeltaSeconds :type "Float (single-precision)"))
  (bind (_hitresult _returnvalue) (`self.GetHitResultUnderCursorByChannel` "TraceTypeQuery1"))
  (bind (_bblockinghit _binitialoverlap _time _distance _location) (`GameplayStatics.BreakHitResult` _hitresult))
  ;[1 1 1] Example of how to calculate start and end poit of the movement
  ;;[0.5336 0.3481 1] Ref to the PathPreviewComponent filled inside the BP_Character
  (`self.PathPreviewComp`
    (:`then`
      (if (`PathPreviewComponent.AlwaysShow` (`self.PathPreviewComp`))
        (if _returnvalue
          (if (>= (`KismetMathLibrary.Vector_Distance` _location (`self.PreviousMouseLoc`)) (`self.MinMouseDistanceToRedrawPath`))
            (set `self.PreviousMouseLoc` _location)
            (`PathPreviewComponent.CalculatePathAndShowPreview` (`self.PathPreviewComp`) (`self.K2_GetActorLocation` (`ActorComponent.GetOwner` (`self.PathPreviewComp`))) _location :!label _label_2)))
        (elif (`self.WasInputKeyJustPressed` "SpaceBar")
          (goto _label_2))))
    (:`else`)))

(event `EnhancedInput|/AIPathPreviewComponent/Content/Inputs/IA_MoveX`
  (params (ActionValue :type "Float (double-precision)") (ElapsedSeconds :type "Float (double-precision)") (TriggeredSeconds :type "Float (double-precision)") (InputAction :type "InputAction Object Reference" :default "/AIPathPreviewComponent/Content/Inputs/IA_MoveX.IA_MoveX"))
  (bind _camerapawn (`self.CameraPawn`))
  (:`Triggered`
    (`Pawn.AddMovementInput` _camerapawn (* (`self.GetActorForwardVector` _camerapawn) ActionValue) 100.0 false)
    (`/AIPathPreviewComponent/Content/Blueprints/BP_CameraPawn.CheckHeight` (`self.CameraPawn`))))

(event `EnhancedInput|/AIPathPreviewComponent/Content/Inputs/IA_MoveY`
  (params (ActionValue :type "Float (double-precision)") (ElapsedSeconds :type "Float (double-precision)") (TriggeredSeconds :type "Float (double-precision)") (InputAction :type "InputAction Object Reference" :default "/AIPathPreviewComponent/Content/Inputs/IA_MoveY.IA_MoveY"))
  (bind _camerapawn (`self.CameraPawn`))
  (:`Triggered`
    (`Pawn.AddMovementInput` _camerapawn (* ActionValue (`self.GetActorRightVector` _camerapawn)) 100.0 false)
    (`/AIPathPreviewComponent/Content/Blueprints/BP_CameraPawn.CheckHeight` (`self.CameraPawn`))))

(fn `SetPathPreviewComp`
  (params (PathPreviewComp :type "PathPreviewComponent Object Reference"))
  (set `self.PathPreviewComp` PathPreviewComp))

(fn `UserConstructionScript`)