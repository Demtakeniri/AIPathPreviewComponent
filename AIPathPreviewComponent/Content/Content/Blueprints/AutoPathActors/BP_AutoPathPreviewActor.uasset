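; Preview actor that visualizes an AI controller's current navigation path, with optional world-space text showing path details.
; After a short startup delay, a looping timer polls the path points and passes them to ShowPathPreview.
; The text widget receives the pawn, point count and path length, and moves just above the final point.
; Settings control detail visibility, polling interval and whether the mesh clears when movement completes.
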(event `self.ReceiveBeginPlay`
  (bind _aswbp_world_text (cast `/AIPathPreviewComponent/Content/Widgets/WBP_WorldText` (`WidgetComponent.GetWidget` (`self.WorldText`))))
  (set `self.WorldTextWidgetRef` _aswbp_world_text)
  (if (`/AIPathPreviewComponent/Content/Blueprints/DataAssets/BP_AutoPathPreviewSettings.ClearPathOnMoveCompleted` (`self.AutoPathSettings`))
    (add `AIController.ReceiveMoveCompleted` (`self.AiControllerRef`) (delegate `ClearPathOnMovementCompleted`)))
  (`KismetSystemLibrary.Delay` 0.2)
  (`self.StartShowingPath`))

(event `ClearPathOnMovementCompleted`
  (params (RequestID :type "AIRequestID Structure") (Result :type "EPathFollowingResult Enum" :default "Success"))
  (`self.ClearMesh`))

(event `StartShowingPath`
  (bind _timerhandle (`self.TimerHandle`))
  (bind _returnvalue (`AIBlueprintHelperLibrary.GetCurrentPathPoints` (`self.AiControllerRef`)))
  (if (`KismetSystemLibrary.K2_IsValidTimerHandle` _timerhandle)
    (`KismetSystemLibrary.K2_ClearAndInvalidateTimerHandle` _timerhandle))
  (bind _aicontrollerref (`self.AiControllerRef`)
    (:`then`
      (`/Engine/EditorBlueprintResources/StandardMacros.IsValid` _aicontrollerref
        (:`Is Valid`
          (if (`KismetArrayLibrary.Array_IsNotEmpty` _returnvalue)
            (`self.ShowPathPreview` _returnvalue)
            (`self.ShowDetailsText` _returnvalue)))))
    (:`else`
      _))
  (bind _returnvalue_2 (`KismetSystemLibrary.K2_SetTimerDelegate` (delegate `StartShowingPath`) (`/AIPathPreviewComponent/Content/Blueprints/DataAssets/BP_AutoPathPreviewSettings.TimeBetweenPathChecks` (`self.AutoPathSettings`)) true))
  (set `self.TimerHandle` _returnvalue_2))

(fn `ShowDetailsText`
  (params (Array :type "Array of Vector Structure"))
  (bind _returnvalue (`KismetArrayLibrary.Array_Length` Array))
  (bind _aicontrollerref (`self.AiControllerRef`))
  (`/AIPathPreviewComponent/Content/Widgets/WBP_WorldText.SetText` (`self.WorldTextWidgetRef`) (`Controller.K2_GetPawn` _aicontrollerref) _returnvalue (`NavigationPath.GetPathLength` (`AIBlueprintHelperLibrary.GetCurrentPath` _aicontrollerref)))
  (`SceneComponent.K2_SetWorldLocation` (`self.WorldText`) (`KismetMathLibrary.MakeVector` (.x (`|GetArrayItem` Array (- _returnvalue 1))) (.y (`|GetArrayItem` Array (- _returnvalue 1))) (+ (.z (`|GetArrayItem` Array (- _returnvalue 1))) 50.0)) false true))

(fn `UserConstructionScript`
  (bind _worldtext (`self.WorldText`))
  (`parent.UserConstructionScript`)
  (if (`/AIPathPreviewComponent/Content/Blueprints/DataAssets/BP_AutoPathPreviewSettings.ShowDetails` (`self.AutoPathSettings`))
    (`SceneComponent.SetVisibility` _worldtext true false)
    (else
      (`SceneComponent.SetVisibility` _worldtext false false))))