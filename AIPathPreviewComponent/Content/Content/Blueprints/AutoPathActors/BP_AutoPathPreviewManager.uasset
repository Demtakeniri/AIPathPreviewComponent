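; Manager actor that automatically gives each AI-controlled pawn in the scene a path preview actor.
; On BeginPlay and on a looping timer from Settings, it scans all pawns and spawns a BP_AutoPathPreviewActor for each untracked AI controller.
; A reset event bound through Settings destroys all previews and rescans, while EndPlay just clears them.
; The construction script enforces a single instance by destroying itself if another manager is found.
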(event `self.ReceiveBeginPlay`
  ;[1 1 1] Do a first check and then starts a looping timer
  (add `/AIPathPreviewComponent/Content/Blueprints/DataAssets/BP_AutoPathPreviewSettings.Reset` (`self.Settings`) (delegate `Reset_Event`))
  (`self.CheckPawnsInScene`)
  (bind _returnvalue (`KismetSystemLibrary.K2_SetTimerDelegate` (delegate `OnTImerEnd`) (`/AIPathPreviewComponent/Content/Blueprints/DataAssets/BP_AutoPathPreviewSettings.TimeBetweenAiInSceneCheck` (`self.Settings`)) true))
  (set `self.Timerhandle` _returnvalue))

(event `OnTImerEnd`
  ;[1 1 1] Do a first check and then starts a looping timer
  (`self.CheckPawnsInScene`))

(event `Reset_Event`
  ;[1 1 1] Do a first check and then starts a looping timer
  (`self.DestroyCurrentlySpawnedPathPreviews`)
  (`self.CheckPawnsInScene`))

(event `CheckPawnsInScene`
  ;[1 1 1] Checks the actors in scene to see if there's some with an AiController, then fills an array with all those that do not have a path preview actor yet, then spawns them
  (bind _outactors (`GameplayStatics.GetAllActorsOfClass` "/Script/Engine.Pawn"))
  (for _array_element _outactors
    (bind _returnvalue (`AIBlueprintHelperLibrary.GetAIController` _array_element))
    (`/Engine/EditorBlueprintResources/StandardMacros.IsValid` _returnvalue
      (:`Is Valid`
        (if (not (`KismetArrayLibrary.Array_Contains` (`self.AiControllersArray`) _returnvalue))
          (`KismetArrayLibrary.Array_Add` (`self.AiControllersToSpawn`) _returnvalue)))))
  (`self.SpawnAutoPathPreviewActors`))

(event `SpawnAutoPathPreviewActors`
  (bind _aicontrollerstospawn (`self.AiControllersToSpawn`))
  ;[1 1 1] Cycle the array of AiControllers in order to spawn a path preview actor for each one of them, then clears the array
  (bind (_arrayindex _arrayelement) (`/Engine/EditorBlueprintResources/StandardMacros.ReverseForEachLoop` _aicontrollerstospawn)
    (:`LoopBody`
      (bind _returnvalue (`|SpawnActorFromClass` "/AIPathPreviewComponent/Content/Blueprints/AutoPathActors/BP_AutoPathPreviewActor.BP_AutoPathPreviewActor_C" (`KismetMathLibrary.MakeTransform` (0.0 0.0 0.0)) "Undefined" "MultiplyWithRoot" null _arrayelement null))
      (`KismetArrayLibrary.Array_Add` (`self.SpawnedActors`) _returnvalue)
      (`KismetArrayLibrary.Array_AddUnique` (`self.AiControllersArray`) _arrayelement)
      (`KismetArrayLibrary.Array_RemoveItem` _aicontrollerstospawn _arrayelement))))

(event `self.ReceiveEndPlay`
  (params (EndPlayReason :type "EEndPlayReason Enum" :default "Destroyed"))
  ;[1 1 1] Clears all on end play
  (`self.DestroyCurrentlySpawnedPathPreviews`))

(event `DestroyCurrentlySpawnedPathPreviews`
  (bind _spawnedactors (`self.SpawnedActors`))
  ;[1 1 1] Destrys all the automatic path previews in scene
  (bind (_arrayindex _arrayelement) (`/Engine/EditorBlueprintResources/StandardMacros.ReverseForEachLoop` _spawnedactors)
    (:`LoopBody`
      (`self.K2_DestroyActor` _arrayelement))
    (:`Completed`
      (`KismetArrayLibrary.Array_Clear` _spawnedactors)
      (`KismetArrayLibrary.Array_Clear` (`self.AiControllersArray`)))))

(fn `UserConstructionScript`
  (bind _returnvalue (`GameplayStatics.GetActorOfClass` "BP_AutoPathPreviewManager_C"))
  (if (!= _returnvalue self)
    (`self.K2_DestroyActor`)
    (`KismetSystemLibrary.CollectGarbage`)))